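; BP_Voxel is a voxel terrain actor that renders voxels as instances of an InstancedStaticMesh.
; Its AddInstanceVoxel event places an instance at a given location, lowered by half the voxel size.
; A disconnected, never-executed graph would fill a per-chunk Noise height array from layered 2D simplex noise at several frequencies, offset by chunk index.
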(event `self.AddInstanceVoxel`
  (params (instanceLoc :type "Vector Structure"))
  (`InstancedStaticMeshComponent.AddInstance` (`self.InstancedStaticMesh`) (`KismetMathLibrary.Conv_VectorToTransform` (`KismetMathLibrary.MakeVector` (.x instanceLoc) (.y instanceLoc) (- (.z instanceLoc) (`KismetMathLibrary.Conv_IntToDouble` (/ (`self.VoxelSize`) 2)))))))

(fn `UserConstructionScript`)