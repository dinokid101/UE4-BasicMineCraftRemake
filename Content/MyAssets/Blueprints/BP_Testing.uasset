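; BP_Testing is a test actor that builds a blocky, Minecraft-style terrain patch from instanced static meshes in its Construction Script.
; A nested loop lays out a square grid, setting each instance's height from floored 2D simplex noise for stepped elevation.
; Noise coordinates are offset by the actor's grid-floored world location, so the terrain pattern follows world position.
; The event graph holds only disabled placeholder events.
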(fn `UserConstructionScript`
  (for _index (range 21)
    (for _index_2 (range 21)
      (bind _returnvalue (`SimplexNoiseBPLibrary.SimplexNoise2D` (* (+ _index (`KismetMathLibrary.FFloor` (.x (/ (`self.K2_GetActorLocation`) 100.0)))) 0.01) (* (+ _index_2 (`KismetMathLibrary.FFloor` (.y (/ (`self.K2_GetActorLocation`) 100.0)))) 0.01)))
      (`InstancedStaticMeshComponent.AddInstance` (`self.InstancedStaticMesh`) (`KismetMathLibrary.Conv_VectorToTransform` (`KismetMathLibrary.MakeVector` (* _index 100.0) (* _index_2 100.0) (* (`KismetMathLibrary.Conv_IntToDouble` (`KismetMathLibrary.FFloor` (* _returnvalue 20.0))) 100.0)))))))